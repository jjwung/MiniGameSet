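; Shooter scene component that fires pooled bullets from its own world transform.
; SpawnBullet is gated by a CanFire flag, which it clears and restores after a delay inversely proportional to ShootRate.
; Each shot acquires a BulletClass actor from the ActorPoolSubsystem, calls InitEvent on it as a BP_BulletBase, then plays ShootSound at the component's location.
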(event `Spawn Bullet`
  (bind _returnvalue (`self.K2_GetComponentToWorld`))
  (if (`self.CanFire`)
    (`|ExecutionSequence`
      (:`then_0`
        (set `self.CanFire` false)
        (`KismetSystemLibrary.Delay` (/ 2.0 (`self.ShootRate`)))
        (set `self.CanFire` true))
      (:`then_1`
        (bind _returnvalue_2 (`ActorPoolSubsystem.AcquireActor` (subsystem `ActorPoolSubsystem`) (`self.BulletClass`) _returnvalue "Undefined"))
        (bind _asbp_bullet_base (cast `/Game/Blueprint/Pawn/BP_BulletBase` _returnvalue_2))
        (`/Game/Blueprint/Pawn/BP_BulletBase.InitEvent` _asbp_bullet_base)
        (`GameplayStatics.PlaySoundAtLocation` (`self.ShootSound`) (.location _returnvalue) (struct) 1.0 1.0 0.0 null null null null)))))