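; BP_Missile is a missile actor that tracks nearby pawns and decoy projectiles as scan candidates.
; Its collision sphere's begin and end overlap events add and remove BP_Pawn and BP_DecoyProjectile actors in ScanActors.
; Each Tick runs a debug-drawn visibility trace from every scanned actor to the Head component, without using the result.
; BeginPlay prints the overlapping pawn count, noted as not working; no movement or homing logic is present.
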(event `self.ReceiveBeginPlay`
  (`KismetSystemLibrary.PrintString` (`KismetStringLibrary.Conv_IntToString` (`KismetArrayLibrary.Array_Length` (`PrimitiveComponent.GetOverlappingActors` (`self.CollistionSphere`) "/Game/Blueprint/Pawn/BP_Pawn.BP_Pawn_C"))) true true (struct :`R` 1.0 :`G` 0.311278 :`A` 1.0)) ; 不生效
)

(event `self.CollistionSphere.OnComponentBeginOverlap`
  (params (OverlappedComponent :type "PrimitiveComponent Object Reference") (OtherActor :type "Actor Object Reference") (OtherComp :type "PrimitiveComponent Object Reference") (OtherBodyIndex :type Integer) (bFromSweep :type Boolean) (SweepResult :type "HitResult Structure (by ref)"))
  (cast `/Game/Blueprint/Pawn/BP_Pawn` OtherActor
    (:`then`
      _)
    (:`CastFailed`
      (cast `/Game/Blueprint/Actor/BP_DecoyProjectile` OtherActor)))
  (`KismetArrayLibrary.Array_Add` (`self.ScanActors`) OtherActor))

(event `self.CollistionSphere.OnComponentEndOverlap`
  (params (OverlappedComponent :type "PrimitiveComponent Object Reference") (OtherActor :type "Actor Object Reference") (OtherComp :type "PrimitiveComponent Object Reference") (OtherBodyIndex :type Integer))
  (cast `/Game/Blueprint/Pawn/BP_Pawn` OtherActor
    (:`then`
      _)
    (:`CastFailed`
      (cast `/Game/Blueprint/Actor/BP_DecoyProjectile` OtherActor)))
  (`KismetArrayLibrary.Array_RemoveItem` (`self.ScanActors`) OtherActor))

(event `self.ReceiveTick`
  (params (DeltaSeconds :type "Float (single-precision)"))
  (for _array_element (`self.ScanActors`)
    (`KismetSystemLibrary.LineTraceSingle` :`Start` (`self.K2_GetActorLocation` _array_element) :`End` (`SceneComponent.K2_GetComponentLocation` (`self.Head`)) :`TraceChannel` "TraceTypeQuery1" :`DrawDebugType` "ForOneFrame")))

(fn `UserConstructionScript`)