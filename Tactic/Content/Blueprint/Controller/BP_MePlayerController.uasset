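; BP_MePlayerController is a player controller that turns the controlled BP_Pawn according to the mouse position on screen.
; Every Tick it casts the controlled pawn to BP_Pawn and passes it the rotation from GetMouseRotation.
; That function scales the viewport mouse position by the viewport scale and derives a yaw-only rotation from its angle to the screen center, with no world trace.
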(event `self.ReceiveTick`
  (params (DeltaSeconds :type "Float (single-precision)"))
  (bind _asbp_pawn (cast `/Game/Blueprint/Pawn/BP_Pawn` (`self.K2_GetPawn`)))
  (`/Game/Blueprint/Pawn/BP_Pawn.SetPawnRotation` _asbp_pawn (`self.GetMouseRotation`)))

(fn `GetMouseRotation`
  (returns (ReturnValue :type "Rotator Structure"))
  (bind _returnvalue (`WidgetLayoutLibrary.GetMousePositionOnViewport`))
  (return (`KismetMathLibrary.MakeRotator` 0.0 0.0 (`TacticToolFunction.CalculateMouseAngleToCenter` (* _returnvalue (`WidgetLayoutLibrary.GetViewportScale`)) (`WidgetLayoutLibrary.GetViewportSize`)))))

(fn `UserConstructionScript`)