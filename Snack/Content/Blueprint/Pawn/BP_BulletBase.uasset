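; Base pooled bullet that flies straight along its forward vector and detects hits on pawns of other groups.
; InitEvent opens a Tick gate, then after a fixed delay closes it and releases the actor to the ActorPoolSubsystem.
; Movement is an unswept per-frame offset, not scaled by delta time.
; CheckBox overlaps filter BP_Pawns by Group but only print a hit message; Move is an empty stub.
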(event `InitEvent`
  (`self.StartMoving` (`self.Speed`))
  (`KismetSystemLibrary.Delay` 10.0)
  (`self.StopMoving`)
  (`ActorPoolSubsystem.ReleaseActor` (subsystem `ActorPoolSubsystem`) self))

(event `self.ReceiveTick`
  (params (DeltaSeconds :type "Float (single-precision)"))
  (`/Engine/EditorBlueprintResources/StandardMacros.Gate` true :!label _label
    (:`Exit`
      (`self.K2_AddActorWorldOffset` (* (`self.GetActorForwardVector`) (stale `StartMoving` Speed))))))

(event `StartMoving`
  (params (Speed :type "Float (double-precision)"))
  (goto _label :!via `Open`))

(event `StopMoving`
  (goto _label :!via `Close`))

(event `self.CheckBox.OnComponentBeginOverlap`
  (params (OverlappedComponent :type "PrimitiveComponent Object Reference") (OtherActor :type "Actor Object Reference") (OtherComp :type "PrimitiveComponent Object Reference") (OtherBodyIndex :type Integer) (bFromSweep :type Boolean) (SweepResult :type "HitResult Structure (by ref)"))
  (bind _asbp_pawn (cast `/Game/Blueprint/Pawn/BP_Pawn` OtherActor))
  (bind _group (`/Game/Blueprint/Pawn/BP_Pawn.Group` _asbp_pawn))
  (if (and (`|EnumInequality` _group "NewEnumerator0") (`|EnumInequality` _group (`self.Group`)))
    (`KismetSystemLibrary.PrintString` "击中")))

(fn `Move`)

(fn `UserConstructionScript`)