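; BP_Food is a food pickup actor that relocates when a BP_Snack actor touches it.
; Its Sphere overlap event proceeds only if the other actor is BP_Snack and the overlapping component is a sphere, then calls SpawnNewFood.
; SpawnNewFood reuses the same actor, moving it by a random X/Y offset from its current position at a fixed height, without sweeping.
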(event `self.Sphere.OnComponentBeginOverlap`
  (params (OverlappedComponent :type "PrimitiveComponent Object Reference") (OtherActor :type "Actor Object Reference") (OtherComp :type "PrimitiveComponent Object Reference") (OtherBodyIndex :type Integer) (bFromSweep :type Boolean) (SweepResult :type "HitResult Structure (by ref)"))
  (cast `/Game/Blueprints/BP_Snack` OtherActor)
  (cast `SphereComponent` OtherComp)
  (`self.SpawnNewFood`))

(event `SpawnNewFood`
  (bind (_returnvalue_x _returnvalue_y) (`KismetMathLibrary.BreakVector` (`self.K2_GetActorLocation`)))
  (`self.K2_SetActorLocation` (`KismetMathLibrary.MakeVector` (+ _returnvalue_x (`KismetMathLibrary.RandomFloatInRange` -500.0 500.0)) (+ _returnvalue_y (`KismetMathLibrary.RandomFloatInRange` -500.0 500.0)) 100.0)))

(fn `UserConstructionScript`)