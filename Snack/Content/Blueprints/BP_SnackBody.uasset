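; BP_SnackBody is a body segment actor that follows transforms supplied by its SnackBase, apparently as part of a snake-like chain.
; Each Tick passes through a gate that StartMove opens.
; While the gate is open and SnackBase is valid, it gets its transform from SnackBase.FindBodyTransform, applies it without sweep or teleport, then calls InsideNext.
; An unconnected debug print of GetNodeTransform remains in the graph.
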(event `self.ReceiveBeginPlay`)

(event `self.ReceiveTick`
  (params (DeltaSeconds :type "Float (single-precision)"))
  (`|ExecutionSequence`
    (:`then_1`
      (`/Engine/EditorBlueprintResources/StandardMacros.Gate` true :!label _label
        (:`Exit`
          (bind _snackbase (`self.SnackBase`)
            (:`then`
              (`self.move` (`SnackBase.FindBodyTransform` _snackbase self))
              (`self.InsideNext`))
            (:`else`)))))))

(event `StartMove`
  (goto _label :!via `Open`))

(event `move`
  (params (Transform :type "Transform Structure"))
  (`self.K2_SetActorTransform` Transform))

(fn `UserConstructionScript`)