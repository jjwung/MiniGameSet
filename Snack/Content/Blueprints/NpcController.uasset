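; NPC controller that makes a possessed BP_Snack wander randomly.
; It stores the snack on possess and clears it on unpossess, while a looping one-second delay from BeginPlay rerolls a random 2D input vector.
; Each Tick feeds that vector into the snack's TriggerMoveEvent, simulating movement input, and prints it or an invalid-reference message for debugging.
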(event `self.ReceivePossess`
  (params (PossessedPawn :type "Pawn Object Reference"))
  (bind _asbp_snack (cast `/Game/Blueprints/BP_Snack` PossessedPawn))
  (set `self.ControlNpcSnack` _asbp_snack))

(event `self.ReceiveUnPossess`
  (params (UnpossessedPawn :type "Pawn Object Reference"))
  (cast `/Game/Blueprints/BP_Snack` UnpossessedPawn)
  (set `self.ControlNpcSnack` null))

(event `self.ReceiveBeginPlay`
  (`|ExecutionSequence`
    (:`then_1`
      (`KismetSystemLibrary.Delay` 1.0 :!label _label)
      (set `self.ActionValue2D` (`KismetMathLibrary.MakeVector2D` (`KismetMathLibrary.RandomFloatInRange` -1.0 1.0) (`KismetMathLibrary.RandomFloatInRange` -1.0 1.0)))
      (goto _label))))

(event `self.ReceiveTick`
  (params (DeltaSeconds :type "Float (single-precision)"))
  (bind _actionvalue2d (`self.ActionValue2D`))
  (bind _controlnpcsnack (`self.ControlNpcSnack`)
    (:`then`
      (`/Game/Blueprints/BP_Snack.TriggerMoveEvent` _controlnpcsnack _actionvalue2d)
      (`KismetSystemLibrary.PrintString` (`KismetStringLibrary.Conv_Vector2dToString` _actionvalue2d) true true (struct :`G` 0.66 :`B` 1.0 :`A` 1.0) 0.0))
    (:`else`
      (`KismetSystemLibrary.PrintString` "无效" true true (struct :`R` 1.0 :`B` 0.079394 :`A` 1.0) 0.0))))

(fn `UserConstructionScript`)