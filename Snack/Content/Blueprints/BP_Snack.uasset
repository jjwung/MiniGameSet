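; Player-controlled head of a snake game that moves continuously, eats food and grows.
; Enhanced Input turns an arrow component, and each tick moves the head along it without delta-time scaling, recording a transform node.
; Mouth overlap with food increases Size and chains a new body segment to the last, starting it after a speed-based delay.
; Growth also raises speed, widens the orthographic camera and updates the HUD; body hits only print.
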(event `Grow`
  (params (GrowSize :type Integer))
  (set `self.Size` (+ GrowSize (`self.Size`)))
  (`self.SpawnBodyAndAttach`))

(event `Key|Two`
  (params (Key :type "Key Structure"))
  (:`Pressed`
    (for _ (range 6)
      (`KismetSystemLibrary.Delay` 1.0)
      (`KismetSystemLibrary.PrintString` "Hello"))))

(event `self.ReceiveBeginPlay`
  (`|ExecutionSequence`
    (:`then_0`
      (bind _returnvalue (`|CreateWidget` "/Game/UI/W_SnakeState.W_SnakeState_C"))
      (bind _output_get (set `self.SnakeStateUI` _returnvalue))
      (`UserWidget.AddToViewport` _output_get 0))
    (:`then_1`
      (bind _assnake_game_instance (cast `/Game/Blueprints/SnakeGameInstance` (`GameplayStatics.GetGameInstance`)))
      (`/Game/Blueprints/SnakeGameInstance.SpawnManyFood` _assnake_game_instance 1000))
    (:`then_2`
      (bind `_as玩家控制器` (cast `PlayerController` (`Pawn.GetController`)))
      (bind _returnvalue_2 (pcsubsystem `EnhancedInputLocalPlayerSubsystem` `_as玩家控制器`))
      (`/Engine/EditorBlueprintResources/StandardMacros.IsValid` _returnvalue_2
        (:`Is Valid`
          (`EnhancedInputSubsystemInterface.AddMappingContext` _returnvalue_2 "/Game/Input/IMC_Default.IMC_Default" 0 (struct)))))))

(event `automove`
  (bind _speed (`self.Speed`))
  (bind (_returnvalue_x _returnvalue_y) (`KismetMathLibrary.BreakVector` (`SceneComponent.GetForwardVector` (`self.ArrowDirection`))))
  (`self.K2_AddActorWorldOffset` (`KismetMathLibrary.MakeVector` (* _returnvalue_x _speed) (* _returnvalue_y _speed))))

(event `self.ReceiveTick`
  (params (DeltaSeconds :type "Float (single-precision)"))
  (`self.automove`)
  (`self.RememberTransforms`))

(event `EnhancedInput|/Game/Input/Actions/IA_Move`
  (params (ActionValue :type "Vector2D Structure") (ElapsedSeconds :type "Float (double-precision)") (TriggeredSeconds :type "Float (double-precision)") (InputAction :type "InputAction Object Reference" :default "/Game/Input/Actions/IA_Move.IA_Move"))
  (bind (_x _y) (`KismetMathLibrary.BreakVector2D` ActionValue))
  (:`Triggered`
    (`SceneComponent.K2_SetRelativeRotation` (`self.ArrowDirection`) (`KismetMathLibrary.Conv_VectorToRotator` (`KismetMathLibrary.MakeVector` _x _y)) false false)))

(event `SpawnBodyAndAttach`
  (bind _body (`self.Body`))
  (bind _returnvalue (`|SpawnActorFromClass` "/Game/Blueprints/BP_SnackBody.BP_SnackBody_C" (`KismetMathLibrary.MakeTransform` (0.0 0.0 100000.0)) "AlwaysSpawn" "MultiplyWithRoot" null null))
  (set `SnackBodyBase.SnackBase` self _returnvalue)
  (`SnackBodyBase.SetHeadNode` _returnvalue (`|GetArrayItem` _body (- (`KismetArrayLibrary.Array_Length` _body) 1)))
  (`KismetArrayLibrary.Array_Add` (`self.Body`) _returnvalue)
  (`KismetSystemLibrary.Delay` (/ 0.1 (`self.Speed`)))
  (`/Game/Blueprints/BP_SnackBody.StartMove` _returnvalue)
  (`self.NextNode`)
  (set `self.Speed` (+ (`self.Speed`) 0.01))
  (`CameraComponent.SetOrthoWidth` (`self.Camera`) (`KismetMathLibrary.Lerp` 3000.0 10000.0 (`KismetMathLibrary.NormalizeToRange` (`self.Speed`) 1.0 10.0)))
  (`/Game/UI/W_SnakeState.SetMass` (`self.SnakeStateUI`) (`self.Size`)))

(event `self.Mouse.OnComponentBeginOverlap`
  (params (OverlappedComponent :type "PrimitiveComponent Object Reference") (OtherActor :type "Actor Object Reference") (OtherComp :type "PrimitiveComponent Object Reference") (OtherBodyIndex :type Integer) (bFromSweep :type Boolean) (SweepResult :type "HitResult Structure (by ref)"))
  (bind _asbp_food (cast `/Game/Blueprints/BP_Food` OtherActor)
    (:`then`
      (`self.Grow` (`/Game/Blueprints/BP_Food.Energy` _asbp_food))
      (`GameplayStatics.PlaySound2D` "/Engine/VREditor/Sounds/VR_ungrab.VR_ungrab" 1.0 1.0 0.0 null null))
    (:`CastFailed`
      (cast `/Game/Blueprints/BP_SnackBody` OtherActor)
      (`KismetSystemLibrary.PrintString` "sw"))))

(fn `RememberTransforms`
  (`self.AddNode` (`KismetMathLibrary.MakeTransform` (`SceneComponent.K2_GetComponentLocation` (`self.Sphere`)) (`SceneComponent.K2_GetComponentRotation` (`self.ArrowDirection`)))))

(fn `UserConstructionScript`)