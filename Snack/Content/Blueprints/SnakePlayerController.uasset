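; Player controller for a snake game that passes player movement input to the snake and shows its state UI.
; Possess caches the pawn as a BP_Snack, and UnPossess clears that reference when the released pawn is a snake.
; The Enhanced Input IA_Move action forwards its value to the cached snake's TriggerMoveEvent while the reference is valid.
; BeginPlay creates the W_SnakeState widget and adds it to the viewport.
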(event `self.ReceivePossess`
  (params (PossessedPawn :type "Pawn Object Reference"))
  (bind _asbp_snack (cast `/Game/Blueprints/BP_Snack` PossessedPawn))
  (set `self.As BP Snack` _asbp_snack))

(event `self.ReceiveUnPossess`
  (params (UnpossessedPawn :type "Pawn Object Reference"))
  (cast `/Game/Blueprints/BP_Snack` UnpossessedPawn)
  (set `self.As BP Snack` null))

(event `EnhancedInput|/Game/Input/Actions/IA_Move`
  (params (ActionValue :type "Vector2D Structure") (ElapsedSeconds :type "Float (double-precision)") (TriggeredSeconds :type "Float (double-precision)") (InputAction :type "InputAction Object Reference" :default "/Game/Input/Actions/IA_Move.IA_Move"))
  (:`Triggered`
    (bind _as_bp_snack (`self.As BP Snack`)
      (:`then`
        (`/Game/Blueprints/BP_Snack.TriggerMoveEvent` _as_bp_snack ActionValue))
      (:`else`))))

(event `self.ReceiveBeginPlay`
  (`|ExecutionSequence`
    (:`then_0`
      ;[0.2686 0.6806 1] 初始化UI
      (bind _returnvalue (`|CreateWidget` "/Game/UI/W_SnakeState.W_SnakeState_C"))
      (bind _output_get (set `self.SnakeStateUI` _returnvalue))
      (`UserWidget.AddToViewport` _output_get 0))))

(fn `UserConstructionScript`)